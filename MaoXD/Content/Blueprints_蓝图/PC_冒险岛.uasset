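; Player controller for the Adventure Island game (冒险岛), handling character selection, pawn spawning and HUD updates.
; On BeginPlay a CL-prefixed client event adds the character selection widget to the viewport and creates the main widget.
; Selection passes through an SRV-prefixed server event to the game mode via interface messages, while a separate event spawns and possesses the chosen pawn.
; Health bar and experience updates reach the main widget through CL events.
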(event Custom|CL_更新健康栏
  (params (百分比 :type Float%20%28single-precision%29) (敌人名称 :type String))
  ;[1 1 1] 更新健康栏
  (Default|更新健康 (Variables|Default|GetWB_主) 百分比 敌人名称))

(event Custom|CL_更新经验
  (params (玩家信息 :type ST%20玩家信息%20Structure))
  ;[1 1 1] 更新经验
  (Default|更新经验 (Variables|Default|GetWB_主) 玩家信息))

(event Custom|SRV_选择玩家
  (params (玩家 :type Actor%20Class%20Reference) (生成位置 :type Vector))
  ;[1 1 1] 界面选择玩家
  (bind _游戏模式 (Class|INT游戏模式|获取游戏模式实例(Message) (Game|GetGameMode)))
  (Class|INT游戏模式|请求生成玩家(Message) _游戏模式 self 玩家 生成位置))

(event Custom|CL_初始化小部件
  ;[1 1 1] 初始化控件
  (bind _returnvalue (UserInterface|CreateWidget "/Game/UI_界面/WB_角色选择.WB_角色选择_C")) ; 创建控件
  (bind _output_get (Variables|Default|SetWB_玩家选择 _returnvalue))
  (UserInterface|Viewport|AddtoViewport _output_get 0)
  (bind _returnvalue_2 (UserInterface|CreateWidget "/Game/UI_界面/WB_主.WB_主_C"))
  (Variables|Default|SetWB_主 _returnvalue_2))

(event EventBeginPlay
  ;[1 1 1] 开始运行
  (CallFunction|初始化小部件))

(event Event初始化小部件
  ;[1 1 1] 初始化控件
  (CallFunction|CL初始化小部件))

(event Event选择玩家
  (params (玩家 :type Actor%20Class%20Reference) (生成位置 :type Vector :default "0, 0, 0"))
  ;[1 1 1] 界面选择玩家
  (CallFunction|SRV选择玩家 玩家 生成位置))

(event Event生成玩家
  (params (玩家 :type Actor%20Class%20Reference) (生成变换 :type Transform))
  ;[1 1 1] 生成玩家
  (bind _returnvalue (Game|SpawnActorfromClass 玩家 生成变换 "AdjustIfPossibleButAlwaysSpawn" 0 0))
  (bind _玩家 (Class|INT玩家基地|获取玩家实例(Message) _returnvalue))
  (Pawn|Possess _玩家))

(event Event更新健康栏
  (params (百分比 :type Float%20%28double-precision%29) (敌人名称 :type String))
  ;[1 1 1] 更新健康栏
  (CallFunction|CL更新健康栏 百分比 敌人名称))

(event Event更新经验
  (params (玩家信息 :type ST%20玩家信息%20Structure))
  ;[1 1 1] 更新经验
  (CallFunction|CL更新经验 玩家信息))

(fn ConstructionScript)

(fn 获取玩家控制器实例
  (return self))