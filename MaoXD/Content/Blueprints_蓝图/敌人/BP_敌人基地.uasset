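; Base networked Paper2D enemy that damages overlapping players, reacts to hits and respawns after death.
; Hits pause AI and movement for the flipbook's length, then the enemy shuttles around the attacker via AIMoveTo until that player dies.
; Death grants XP, fades the sprite, then respawns it at a random navmesh point and restarts the behavior tree.
; Server events set state, with RepNotifies updating flipbook, material, color and location; contact damage runs on a looping timer.
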(event OnComponentBeginOverlap(碰撞)
  (params (OverlappedComponent :type Primitive%20Component%20Object%20Reference) (OtherActor :type Actor%20Object%20Reference) (OtherComp :type Primitive%20Component%20Object%20Reference) (OtherBodyIndex :type Integer) (bFromSweep :type Boolean) (SweepResult :type Hit%20Result%20Structure%20%28by%20ref%29))
  ;[1 1 1] 碰撞/重叠
  (Networking|SwitchHasAuthority
    (:Authority
      (if (Actor|ActorHasTag OtherActor "玩家")
        (CallFunction|开始施加伤害 true)))))

(event OnComponentEndOverlap(碰撞)
  (params (OverlappedComponent :type Primitive%20Component%20Object%20Reference) (OtherActor :type Actor%20Object%20Reference) (OtherComp :type Primitive%20Component%20Object%20Reference) (OtherBodyIndex :type Integer))
  ;[1 1 1] 碰撞/重叠
  (Networking|SwitchHasAuthority
    (:Authority
      (if (Actor|ActorHasTag OtherActor "玩家")
        (CallFunction|开始施加伤害 false)))))

(event Custom|SRV_开始施加伤害
  (params (施加伤害 :type Boolean))
  ;[1 1 1] 对玩家进行伤害
  (if 施加伤害
    (bind _returnvalue (Utilities|Time|SetTimerbyEvent (delegate Custom|应用伤害) 0.1 true))
    (Variables|Default|Set应用伤害句柄 _returnvalue)
    (else
      (Utilities|Time|ClearandInvalidateTimerbyHandle (Variables|Default|Get应用伤害句柄)))))

(event Custom|SRV_设置移动状态
  (params (运动状态 :type E_运动状态%20Enum :default "NewEnumerator0"))
  ;[1 1 1] 运动状态
  (Variables|Default|Set运动状态 运动状态))

(event Custom|应用伤害
  ;[1 1 1] 对玩家进行伤害
  (for _array_element (Collision|GetOverlappingActors "/Game/Blueprints_蓝图/玩家/BP_玩家基地.BP_玩家基地_C" :!class /Script/Engine.Actor)
    (bind _玩家 (Class|INT玩家基地|获取玩家实例(Message) _array_element))
    (if (not (Variables|/Game/Blueprints_蓝图/玩家/BP_玩家基地.BP_玩家基地_C|Get无敌模式 _玩家))
      (Game|Damage|ApplyDamage _玩家 (.伤害 (Utilities|Struct|BreakST_敌人信息 (Variables|Default|Get敌人信息))) (Pawn|GetController) 0 "/Script/Engine.DamageType"))))

(event Custom|SRV_死亡
  (params (已死亡 :type Boolean))
  (bind _output_get (Variables|Default|Set已死亡 已死亡))
  (if _output_get
    (CallFunction|MC死亡 (.死亡音效 (Utilities|Struct|BreakST_敌人信息 (Variables|Default|Get敌人信息))) (Transformation|GetActorLocation))))

(event Custom|SRV_重新生成
  (bind _returnvalue (Actor|GetActorOfClass "/Script/NavigationSystem.NavMeshBoundsVolume"))
  (Variables|Default|Set重新生成位置 (Math|Vector|MakeVector (.X (Math|Vector|BreakVector (.RandomLocation (AI|Navigation|GetRandomReachablePointinRadius (Transformation|GetActorLocation) (.X (Math|Vector|BreakVector (.BoxExtent (Collision|GetActorBounds _returnvalue false false)))) 0 0)))) (.Y (Math|Vector|BreakVector (Transformation|GetActorLocation))) (+ (.Z (Math|Vector|BreakVector (.RandomLocation (AI|Navigation|GetRandomReachablePointinRadius (Transformation|GetActorLocation) (.X (Math|Vector|BreakVector (.BoxExtent (Collision|GetActorBounds _returnvalue false false)))) 0 0)))) 2e+01))))

(event Custom|SRV_Actor褪色
  (params (褪色 :type Boolean))
  (bind _output_get (Variables|Default|Set褪色 褪色))
  (if _output_get
    (bind _褪色通道 (Timeline|褪色Actor PlayFromStart)
      (:Update
        (Variables|Default|SetActor褪色颜色 (Math|Color|Lerp(LinearColor) "(R=1.000000,G=1.000000,B=1.000000,A=1.000000)" "(R=1.000000,G=1.000000,B=1.000000,A=0.000000)" _褪色通道)))
      (:Finished
        (if (not (Variables|Default|Get褪色))
          (CallFunction|死亡 false)
          (CallFunction|重新启动行为树))))
    (else
      (Timeline|褪色Actor ReverseFromEnd))))

(event Custom|MC_死亡
  (params (死亡音效 :type Sound%20Base%20Object%20Reference) (位置 :type Vector))
  (Audio|PlaySoundatLocation 死亡音效 位置 "0, 0, 0" 1.0 1.0 0.0 0 0 0 0))

(event Custom|CL_重新启动行为树
  (Components|Movement|StopMovementImmediately (Variables|Character|GetCharacterMovement))
  (AI|Logic|StopLogic (Variables|/Script/AIModule.AIController|GetBrainComponent (AI|GetAIController self)) "")
  (bind _ai控制器 (Class|INTAI控制器|获取AI控制器实例(Message) (AI|GetAIController self)))
  (Class|INTAI控制器|运行行为树(Message) _ai控制器))

(event Game|Damage|EventAnyDamage
  (params (Damage :type Float%20%28single-precision%29) (DamageType :type Damage%20Type%20Object%20Reference) (InstigatedBy :type Controller%20Object%20Reference) (DamageCauser :type Actor%20Object%20Reference))
  (bind _returnvalue (Transformation|GetActorLocation))
  (bind (_x _y _z) (Math|Vector|BreakVector _returnvalue))
  ;[1 1 1] 接受来自玩家的伤害,并围绕着玩家移动
  (Variables|Default|Set玩家伤害数量 Damage)
  (CallFunction|显示浮动文本 self "NewEnumerator0")
  (Variables|Default|Set玩家控制器 InstigatedBy)
  (bind _structout (Utilities|Struct|SetmembersinST_敌人信息 (Variables|Default|Get敌人信息) (Math|Float|Clamp(Float) (- (Utilities|Struct|BreakST_敌人信息 (Variables|Default|Get敌人信息)) Damage) 0.0 (Utilities|Struct|BreakST_敌人信息 (Variables|Default|Get敌人信息)))))
  (bind _output_get (Variables|Default|Set敌人信息 _structout))
  (Pawn|Components|CharacterMovement|SetMovementMode (Variables|Character|GetCharacterMovement) "MOVE_None" 0) ; 击中无法移动
  (CallFunction|设置运动状态 "NewEnumerator7") ; 击中动画设置
  (AI|Logic|StopLogic (Variables|/Script/AIModule.AIController|GetBrainComponent (AI|GetAIController self)) "击中")
  (Utilities|FlowControl|Delay (Class|PaperFlipbookComponent|GetFlipbookLength (Variables|Default|GetSprite)))
  (if (== (Utilities|Struct|BreakST_敌人信息 _output_get) 0.0)
    (bind _玩家 (Class|INT玩家基地|获取玩家实例(Message) (Pawn|GetControlledPawn (Variables|Default|Get玩家控制器))))
    (Class|INT玩家基地|添加经验(Message) _玩家 (Utilities|Struct|BreakST_敌人信息 (Variables|Default|Get敌人信息)))
    (CallFunction|死亡 true)
    (Variables|/Script/Engine.PrimitiveComponent|SetbGenerateOverlapEvents (Variables|Default|Get命中碰撞) false)
    (Variables|/Script/Engine.PrimitiveComponent|SetbGenerateOverlapEvents (Variables|Default|Get碰撞) false)
    (CallFunction|Actor褪色 true)
    (Utilities|FlowControl|Delay (Variables|Default|Get重新启动计时器))
    (bind _structout_2 (Utilities|Struct|SetmembersinST_敌人信息 (Variables|Default|Get敌人信息) (Utilities|Struct|BreakST_敌人信息 (Variables|Default|Get敌人信息))))
    (Variables|Default|Set敌人信息 _structout_2)
    (Variables|/Script/Engine.PrimitiveComponent|SetbGenerateOverlapEvents (Variables|Default|Get命中碰撞) true)
    (Variables|/Script/Engine.PrimitiveComponent|SetbGenerateOverlapEvents (Variables|Default|Get碰撞) true)
    (Pawn|Components|CharacterMovement|SetMovementMode (Variables|Character|GetCharacterMovement) "MOVE_Walking" 0) ; 重新设置移动
    (CallFunction|设置运动状态 "NewEnumerator1")
    (CallFunction|重新生成)
    (CallFunction|Actor褪色 false)
    (CallFunction|重新启动行为树)
    (else
      (Pawn|Components|CharacterMovement|SetMovementMode (Variables|Character|GetCharacterMovement) "MOVE_Walking" 0) ; 重新设置移动
      (CallFunction|设置运动状态 "NewEnumerator1")
      (AI|AIMoveTo self (Transformation|GetActorLocation (Pawn|GetControlledPawn (Variables|Default|Get玩家控制器))) (Pawn|GetControlledPawn (Variables|Default|Get玩家控制器)) 2.0 false :!label _label
        (:OnSuccess
          (bind _玩家_2 (Class|INT玩家基地|获取玩家实例(Message) (Pawn|GetControlledPawn (Variables|Default|Get玩家控制器))))
          (if (not (Variables|/Game/Blueprints_蓝图/玩家/BP_玩家基地.BP_玩家基地_C|Get是死亡 _玩家_2))
            (AI|AIMoveTo (AI|GetAIController self) (Math|Vector|MakeVector (+ _x (Math|Float|SelectFloat -125.0 125.0 (< (.X (Math|Vector|BreakVector (Transformation|GetActorLocation (Pawn|GetControlledPawn (Variables|Default|Get玩家控制器))))) _x))) _y _z) 0 -1.0 "Default" "Default" true true
              (:OnMoveFinished
                (goto _label)))
            (else
              (CallFunction|重新启动行为树))))))))

(event Event设置运动状态
  (params (运动状态 :type E_运动状态%20Enum :default "NewEnumerator0"))
  ;[1 1 1] 运动状态
  (CallFunction|SRV设置移动状态 运动状态))

(event Event开始施加伤害
  (params (施加伤害 :type Boolean))
  ;[1 1 1] 对玩家进行伤害
  (CallFunction|SRV开始施加伤害 施加伤害))

(event Event死亡
  (params (已死亡 :type Boolean))
  (CallFunction|SRV死亡 已死亡))

(event Event重新生成
  (CallFunction|SRV重新生成))

(event EventActor褪色
  (params (褪色 :type Boolean))
  (CallFunction|SRVActor褪色 褪色))

(event Event重新启动行为树
  (CallFunction|CL重新启动行为树))

(fn ConstructionScript
  (|CallParentFunction))

(fn OnRep正在移动
  (bind _sprite (Variables|Default|GetSprite))
  (bind _敌人信息 (Variables|Default|Get敌人信息))
  (bind (_最大健康 _健康 _伤害 _经验值 _待机动画 _移动动画) (Utilities|Struct|BreakST_敌人信息 _敌人信息))
  (if (not (Variables|Default|Get正在移动)) ; 真[待机]假[移动]
    (Sprite|SetFlipbook _sprite _待机动画)
    (else
      (Sprite|SetFlipbook _sprite _移动动画))))

(fn OnRep运动状态
  (bind _敌人信息 (Variables|Default|Get敌人信息))
  (bind (_经验值 _待机动画 _移动动画 _击中动画 _死亡动画) (Utilities|Struct|BreakST_敌人信息 _敌人信息))
  (switch Utilities|FlowControl|Switch|SwitchonE_运动状态 (Variables|Default|Get运动状态)
    (:NewEnumerator0
      (Sprite|SetFlipbook (Variables|Default|GetSprite) _待机动画))
    (:NewEnumerator1
      (Sprite|SetFlipbook (Variables|Default|GetSprite) _移动动画))
    (:NewEnumerator7
      (Sprite|SetFlipbook (Variables|Default|GetSprite) _击中动画))
    (:NewEnumerator8
      (Sprite|SetFlipbook (Variables|Default|GetSprite) _死亡动画))))

(fn OnRep已死亡
  (if (Variables|Default|Get已死亡)
    (CallFunction|设置运动状态 "NewEnumerator8")
    (Rendering|Material|SetMaterial (Variables|Default|GetSprite) 0 "/Paper2D/TranslucentUnlitSpriteMaterial.TranslucentUnlitSpriteMaterial")
    (else
      (Rendering|Material|SetMaterial (Variables|Default|GetSprite) 0 "/Paper2D/MaskedUnlitSpriteMaterial.MaskedUnlitSpriteMaterial"))))

(fn OnRep重新生成位置
  (Transformation|SetActorLocation (Variables|Default|Get重新生成位置) false false))

(fn OnRepActor褪色颜色
  (Sprite|SetSpriteColor (Variables|Default|GetSprite) (Variables|Default|GetActor褪色颜色)))

(fn 获取敌人实例
  (return self))