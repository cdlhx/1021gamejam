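; BP_角色基地 is a character base Blueprint that shows floating damage text over hurt actors.
; 显示浮动文本 forwards to an SRV-prefixed event, which spawns a BP_浮动文本 actor slightly above the hurt actor.
; A switch on text type reads the damage amount from the hurt enemy or player through instance-getter messages, then sets the text, color and sword or blood icon.
; 获取角色基地实例 returns self.
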(event Custom|SRV_显示浮动文本
  (params (受伤Actor :type Actor%20Object%20Reference) (浮动文本类型 :type E_浮动文本类型%20Enum :default "NewEnumerator0"))
  (bind _output_get (Variables|Default|Set受伤%20Actor 受伤Actor))
  (bind _returnvalue (Game|SpawnActorfromClass "/Game/Blueprints_蓝图/BP_浮动文本.BP_浮动文本_C" (Math|Transform|MakeTransform (Math|Vector|MakeVector (.X (Math|Vector|BreakVector (Transformation|GetActorLocation _output_get))) (.Y (Math|Vector|BreakVector (Transformation|GetActorLocation _output_get))) (+ (.Z (Math|Vector|BreakVector (Transformation|GetActorLocation _output_get))) 3e+01))) "AdjustIfPossibleButAlwaysSpawn" 0 0))
  (bind _output_get_2 (Variables|Default|Set浮动文本 _returnvalue))
  (switch Utilities|FlowControl|Switch|SwitchonE_浮动文本类型 浮动文本类型
    (:NewEnumerator0
      (bind _敌人 (Class|INT敌人基地|获取敌人实例(Message) (Variables|Default|Get受伤%20Actor)))
      (Default|显示浮动文本 _output_get_2 (Utilities|Text|ToText(Float) (Variables|/Game/Blueprints_蓝图/敌人/BP_敌人基地.BP_敌人基地_C|Get玩家伤害数量 _敌人) "HalfToEven") "(R=0.500000,G=0.750000,B=1.000000,A=1.000000)" "/Game/UI_界面/图像/IMG_Sword.IMG_Sword"))
    (:NewEnumerator1
      (bind _玩家 (Class|INT玩家基地|获取玩家实例(Message) (Variables|Default|Get受伤%20Actor)))
      (Default|显示浮动文本 _output_get_2 (Utilities|Text|ToText(Float) (Variables|/Game/Blueprints_蓝图/玩家/BP_玩家基地.BP_玩家基地_C|Get敌人伤害数量 _玩家) "HalfToEven") "(R=1.000000,G=0.500000,B=0.500000,A=1.000000)" "/Game/UI_界面/图像/IMG_Blood.IMG_Blood"))))

(event Event显示浮动文本
  (params (受伤Actor :type Actor%20Object%20Reference) (浮动文本类型 :type E_浮动文本类型%20Enum :default "NewEnumerator0"))
  (CallFunction|SRV显示浮动文本 受伤Actor 浮动文本类型))

(fn ConstructionScript)

(fn 获取角色基地实例
  (return self))