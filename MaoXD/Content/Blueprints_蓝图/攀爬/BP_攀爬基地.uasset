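; BP_攀爬基地 (climbing base) is a climbable actor that tells players when they can climb it.
; On the server only, its collision box watches overlaps from actors tagged 玩家 (player) and fetches the player instance through an interface message.
; Entering sends 可以攀爬 (can climb) as true with itself as the climb target; leaving sends it as false.
; The climbing movement itself is not handled here.
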(event OnComponentBeginOverlap(碰撞盒)
  (params (OverlappedComponent :type Primitive%20Component%20Object%20Reference) (OtherActor :type Actor%20Object%20Reference) (OtherComp :type Primitive%20Component%20Object%20Reference) (OtherBodyIndex :type Integer) (bFromSweep :type Boolean) (SweepResult :type Hit%20Result%20Structure%20%28by%20ref%29))
  (Networking|SwitchHasAuthority
    (:Authority
      (if (Actor|ActorHasTag OtherActor "玩家")
        (bind _玩家 (Class|INT玩家基地|获取玩家实例(Message) OtherActor))
        (Class|INT玩家基地|可以攀爬(Message) _玩家 true self)))))

(event OnComponentEndOverlap(碰撞盒)
  (params (OverlappedComponent :type Primitive%20Component%20Object%20Reference) (OtherActor :type Actor%20Object%20Reference) (OtherComp :type Primitive%20Component%20Object%20Reference) (OtherBodyIndex :type Integer))
  (Networking|SwitchHasAuthority
    (:Authority
      (if (Actor|ActorHasTag OtherActor "玩家")
        (bind _玩家 (Class|INT玩家基地|获取玩家实例(Message) OtherActor))
        (Class|INT玩家基地|可以攀爬(Message) _玩家 false)))))

(fn ConstructionScript)