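; BP_StarBase is a star actor that makes an assigned planet orbit around it.
; Each Tick, UpdatePlanetState registers the star on a valid SuroundPlanet, rotates the planet's offset by SuroundSpeed in yaw, and teleports it there.
; The step is not scaled by delta time, so orbit speed depends on frame rate.
; Turn reverses the orbit by negating SuroundSpeed; a look-at rotation for the planet is left disconnected.
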(event Custom|Update%20Planet%20State
  (bind _returnvalue (Transformation|GetActorLocation))
  (bind _suroundplanet (Variables|Default|GetSuroundPlanet))
  (Utilities|IsValid _suroundplanet
    (:Is%20Valid
      (Default|SetStar (Variables|Default|GetSuroundPlanet) self)
      (Transformation|SetActorLocation (Variables|Default|GetSuroundPlanet) (+ (Math|Vector|RotateVector (- (Transformation|GetActorLocation _suroundplanet) _returnvalue) (Math|Rotator|MakeRotator 0.0 0.0 (Variables|Default|GetSuroundSpeed))) _returnvalue) false true))))

(event EventTick
  (params (DeltaSeconds :type Float%20%28single-precision%29))
  (CallFunction|UpdatePlanetState))

(fn ConstructionScript)

(fn Turn
  (Variables|Default|SetSuroundSpeed (* (Variables|Default|GetSuroundSpeed) -1.0)))