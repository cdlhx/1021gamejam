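; Material component that plays timed flipbook and fade effects on a mesh and serves materials from an array indexed by character state.
; PlayAnim and PlayAnimFade put a dynamic instance of AnimMaterial on the mesh, set up with a frame texture and grid size.
; Tick counts down the timer, driving ImageSpeed for flipbooks or ImageMask for fades.
; When a flipbook ends, a re-armed DoOnce swaps in the follow-up material, if valid.
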(event Custom|PlayAnim
  (params (Time :type Float%20%28double-precision%29) (Row :type Integer) (Col :type Integer) (NewMaterial :type Material%20Instance%20Object%20Reference) (Texture :type Texture%20Object%20Reference) (Geo :type Static%20Mesh%20Component%20Object%20Reference))
  (Variables|Default|SetAnimNum (* Row Col))
  (Variables|Default|SetGeo Geo)
  (bind _returnvalue (Rendering|Material|CreateDynamicMaterialInstance (Variables|Default|GetAnimMaterial) "None" "None" :!class /Script/Engine.KismetMaterialLibrary))
  (bind _output_get (Variables|Default|SetDyMat _returnvalue))
  (Rendering|Material|SetTextureParameterValue _output_get "Frames" Texture)
  (Rendering|Material|SetScalarParameterValue (Variables|Default|GetDyMat) "ImageRow" (Math|Conversions|ToFloat(Integer) Row) :!class /Script/Engine.MaterialInstanceDynamic)
  (Rendering|Material|SetScalarParameterValue (Variables|Default|GetDyMat) "ImageColumns" (Math|Conversions|ToFloat(Integer) Col) :!class /Script/Engine.MaterialInstanceDynamic)
  (Rendering|Material|SetMaterial Geo 0 (Variables|Default|GetDyMat))
  (bind _output_get_2 (Variables|Default|SetAnimTime Time))
  (Variables|Default|SetAnimTime_Max _output_get_2)
  (Variables|Default|SetChangeMat NewMaterial)
  (Variables|Default|SetFade false))

(event Custom|PlayAnimFade
  (params (Time :type Float%20%28double-precision%29) (Geo :type Static%20Mesh%20Component%20Object%20Reference) (Texture :type Texture%20Object%20Reference))
  (bind _output_get (Variables|Default|SetGeo Geo))
  (bind _returnvalue (Rendering|Material|CreateDynamicMaterialInstance (Variables|Default|GetAnimMaterial) "None" "None" :!class /Script/Engine.KismetMaterialLibrary))
  (bind _output_get_2 (Variables|Default|SetDyMat _returnvalue))
  (Rendering|Material|SetTextureParameterValue _output_get_2 "Frames" Texture)
  (Rendering|Material|SetScalarParameterValue (Variables|Default|GetDyMat) "ImageRow" 1.0 :!class /Script/Engine.MaterialInstanceDynamic)
  (Rendering|Material|SetScalarParameterValue (Variables|Default|GetDyMat) "ImageColumns" 1.0 :!class /Script/Engine.MaterialInstanceDynamic)
  (Rendering|Material|SetMaterial _output_get 0 (Variables|Default|GetDyMat))
  (bind _output_get_3 (Variables|Default|SetAnimTime Time))
  (Variables|Default|SetAnimTime_Max _output_get_3)
  (Variables|Default|SetFade true))

(event EventBeginPlay)

(event EventTick
  (params (DeltaSeconds :type Float%20%28single-precision%29))
  (bind _changemat (Variables|Default|GetChangeMat))
  (if (> (Variables|Default|GetAnimTime) 0.0)
    (bind _output_get (Variables|Default|SetAnimTime (- (Variables|Default|GetAnimTime) DeltaSeconds)))
    (if (Variables|Default|GetFade)
      (Rendering|Material|SetScalarParameterValue (Variables|Default|GetDyMat) "ImageMask" (Math|Float|Clamp(Float) (/ _output_get (Variables|Default|GetAnimTime_Max)) 0.0 0.999) :!class /Script/Engine.MaterialInstanceDynamic)
      (else
        (Rendering|Material|SetScalarParameterValue (Variables|Default|GetDyMat) "ImageSpeed" (Math|Float|Clamp(Float) (- 1.0 (/ _output_get (Variables|Default|GetAnimTime_Max))) 0.0 0.999) :!class /Script/Engine.MaterialInstanceDynamic)
        (goto _label Reset)))
    (else
      (Utilities|FlowControl|DoOnce true :!label _label
        (:Completed
          (Utilities|IsValid _changemat
            (:Is%20Valid
              (Rendering|Material|SetMaterial (Variables|Default|GetGeo) 0 _changemat))))))))

(fn GetMaterial
  (params (CharacterState :type E_MaterialType%20Enum :default "NewEnumerator0"))
  (return (Utilities|Array|Get(acopy) (Variables|Default|GetMaterials) (Math|Conversions|ToInteger(Byte) CharacterState))))

(fn SetMaterial
  (params (MaterialState :type Integer) (Mesh :type Static%20Mesh%20Component%20Object%20Reference))
  (Rendering|Material|SetMaterial Mesh 0 (Utilities|Array|Get(acopy) (Variables|Default|GetMaterials) MaterialState))
  (return))

(fn NewFunction
  (CallFunction|PlayAnim 0.0))