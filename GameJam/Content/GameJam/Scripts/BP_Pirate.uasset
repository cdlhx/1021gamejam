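; BP_Pirate is a pirate that destroys normal ships entering its sphere.
; On overlap, it destroys any BP_NormalShip and increments the airship destroy count.
; ReadData extends the parent's data read to size that sphere from the configured pirate destroy radius.
; It hides the inherited GeoFule component at BeginPlay and updates its rotation every tick.
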(event OnComponentBeginOverlap(Sphere)
  (params (OverlappedComponent :type Primitive%20Component%20Object%20Reference) (OtherActor :type Actor%20Object%20Reference) (OtherComp :type Primitive%20Component%20Object%20Reference) (OtherBodyIndex :type Integer) (bFromSweep :type Boolean) (SweepResult :type Hit%20Result%20Structure%20%28by%20ref%29))
  (bind _asbp_normal_ship (Utilities|Casting|CastToBP_NormalShip OtherActor))
  (Actor|DestroyActor _asbp_normal_ship)
  (CallFunction|AddAirShipDestroyCount 1))

(event EventBeginPlay
  (|CallParentFunction)
  (Rendering|SetVisibility (Variables|Default|GetGeoFule) false false))

(event Collision|EventActorBeginOverlap
  (params (OtherActor :type Actor%20Object%20Reference))
  (|CallParentFunction OtherActor) ; 此节点被禁用，将不会被调用。\n从引脚连出引线来编译功能。
)

(event EventTick
  (params (DeltaSeconds :type Float%20%28single-precision%29))
  (|CallParentFunction DeltaSeconds)
  (CallFunction|UpdateRotation))

(fn ConstructionScript
  (|CallParentFunction))

(fn ReadData
  (bind _data (|CallParentFunction))
  (Components|Sphere|SetSphereRadius (Variables|Default|GetSphere) (.Pirate_DestoryShipRadius (Utilities|Struct|BreakST_Ship _data)) true)
  (return _data))