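; Blueprint function library of global shortcuts to the airship destroy count and star value held by BP_MainGameState.
; Functions add to or read the destroy count, and decrement or read the star value.
; Each one casts the current game state to BP_MainGameState, forwards the call to it, and stops if the cast fails.
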(fn AddAirShipDestroyCount
  (params (Delta :type Integer))
  (bind _asbp_main_game_state (Utilities|Casting|CastToBP_MainGameState (Game|GetGameState)))
  (Default|AddAirShipDestroyCount _asbp_main_game_state Delta))

(fn GetAirShipDestroyCount
  (bind _asbp_main_game_state (Utilities|Casting|CastToBP_MainGameState (Game|GetGameState)))
  (return (Default|GetAirShipDestroyCount _asbp_main_game_state)))

(fn DecStar
  (bind _asbp_main_game_state (Utilities|Casting|CastToBP_MainGameState (Game|GetGameState)))
  (CallFunction|DecStar _asbp_main_game_state))

(fn GetStar
  (bind _asbp_main_game_state (Utilities|Casting|CastToBP_MainGameState (Game|GetGameState)))
  (return (Default|GetStar _asbp_main_game_state)))