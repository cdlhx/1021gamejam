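; BP_Edge is a boundary actor that reacts when airships or planets begin overlapping its Box component.
; An airship that is not flagged IsStopPlanet is destroyed through DestoryShip and adds one to the airship destroy count.
; A planet that has a valid star has Turn called on that star.
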(event OnComponentBeginOverlap(Box)
  (params (OverlappedComponent :type Primitive%20Component%20Object%20Reference) (OtherActor :type Actor%20Object%20Reference) (OtherComp :type Primitive%20Component%20Object%20Reference) (OtherBodyIndex :type Integer) (bFromSweep :type Boolean) (SweepResult :type Hit%20Result%20Structure%20%28by%20ref%29))
  (bind _asbp_air_ship_base (Utilities|Casting|CastToBP_AirShipBase OtherActor)
    (:then
      (if (not (Variables|/Game/GameJam/Scripts/BP_AirShipBase.BP_AirShipBase_C|GetIsStopPlanet _asbp_air_ship_base))
        (Default|DestoryShip _asbp_air_ship_base true)
        (CallFunction|AddAirShipDestroyCount 1)))
    (:CastFailed
      (bind _asbp_planet_base (Utilities|Casting|CastToBP_PlanetBase OtherActor))
      (Utilities|IsValid (Default|GetStar _asbp_planet_base)
        (:Is%20Valid
          (Default|Turn (Default|GetStar _asbp_planet_base)))))))

(event EventBeginPlay)

(event Collision|EventActorBeginOverlap
  (params (OtherActor :type Actor%20Object%20Reference)))

(event EventTick
  (params (DeltaSeconds :type Float%20%28single-precision%29)))

(fn ConstructionScript)