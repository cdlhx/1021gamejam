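; BP_BGM is a level actor that handles background music.
; On BeginPlay it assigns its Sound to the Audio component, fades it in through PlaySound, and adds a UI_Tut tutorial widget to the viewport.
; PlaySound and StopSound events fade the audio in or out over a shared FadeTime.
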(event Custom|StopSound
  (Audio|Components|Audio|FadeOut (Variables|Default|GetAudio) (Variables|Default|GetFadeTime) 0.0 "Linear" :!class /Script/Engine.AudioComponent))

(event Custom|PlaySound
  (Audio|Components|Audio|FadeIn (Variables|Default|GetAudio) (Variables|Default|GetFadeTime) 1.0 0.0 "Linear" :!class /Script/Engine.AudioComponent))

(event EventBeginPlay
  (Audio|Components|Audio|SetSound (Variables|Default|GetAudio) (Variables|Default|GetSound))
  (CallFunction|PlaySound)
  (bind _returnvalue (UserInterface|CreateWidget "/Game/GameJam/UI/UI_Tut.UI_Tut_C"))
  (UserInterface|Viewport|AddtoViewport _returnvalue 0))

(event Collision|EventActorBeginOverlap
  (params (OtherActor :type Actor%20Object%20Reference)))

(event EventTick
  (params (DeltaSeconds :type Float%20%28single-precision%29)))

(fn ConstructionScript)