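; BP_SaveGame is a save game Blueprint that records a grade per level and writes it to a save slot.
; SaveLevelGrade sets or appends the grade in its own LevelGrade array, based on an array length check.
; It copies that array into a newly created save object and saves it to the TextName slot.
; The slot is loaded and cast first, but its stored grades are never merged into the saved array.
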(fn SaveLevelGrade
  (params (Level :type Integer) (Grade :type Float%20%28double-precision%29))
  (bind _returnvalue (SaveGame|CreateSaveGameObject "BP_SaveGame_C"))
  (bind _returnvalue_2 (SaveGame|LoadGamefromSlot (Variables|Default|GetTextName)))
  (bind _asbp_save_game (Utilities|Casting|CastToBP_SaveGame _returnvalue_2)
    (:then
      (if (<= Level (Utilities|Array|Length (Variables|BP_SaveGame_C|GetLevelGrade _returnvalue)))
        (Utilities|Array|SetArrayElem (Variables|Default|GetLevelGrade) Level Grade :!label _label)
        (else
          (Utilities|Array|Add (Variables|Default|GetLevelGrade) Grade :!label _label_2))))
    (:CastFailed
      (if (<= 0 (Utilities|Array|Length (Variables|BP_SaveGame_C|GetLevelGrade _asbp_save_game)))
        (goto _label)
        (else
          (goto _label_2)))))
  (Variables|BP_SaveGame_C|SetLevelGrade _returnvalue (Variables|Default|GetLevelGrade))
  (SaveGame|SaveGametoSlot _returnvalue (Variables|Default|GetTextName)))