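; BP_BugHole is a teleport hole that moves any actor entering its sphere to the linked Destination hole.
; The teleport takes the destination's X and Y but keeps the traveller's Z and rotation.
; To prevent bouncing back, it disables overlap events on the destination sphere for a two-second delay, while a DoOnce blocks re-triggering until Reset reopens it afterwards.
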(event OnComponentBeginOverlap(Sphere)
  (params (OverlappedComponent :type Primitive%20Component%20Object%20Reference) (OtherActor :type Actor%20Object%20Reference) (OtherComp :type Primitive%20Component%20Object%20Reference) (OtherBodyIndex :type Integer) (bFromSweep :type Boolean) (SweepResult :type Hit%20Result%20Structure%20%28by%20ref%29))
  (bind _destination (Variables|Default|GetDestination))
  (bind _returnvalue (Transformation|GetActorLocation _destination))
  (Utilities|IsValid (Variables|Default|GetDestination)
    (:Is%20Valid
      (Utilities|FlowControl|DoOnce false
        (:Completed
          (Variables|/Script/Engine.PrimitiveComponent|SetbGenerateOverlapEvents (Variables|BP_BugHole_C|GetSphere (Variables|Default|GetDestination)) false)
          (Transformation|Teleport OtherActor (Math|Vector|MakeVector (.x _returnvalue) (.y _returnvalue) (.z (Transformation|GetActorLocation OtherActor))) (Transformation|GetActorRotation OtherActor))
          (Utilities|FlowControl|Delay 2.0)
          (Variables|/Script/Engine.PrimitiveComponent|SetbGenerateOverlapEvents (Variables|BP_BugHole_C|GetSphere (Variables|Default|GetDestination)) true)
          (CallFunction|Reset))))))

(event Custom|Reset
  (bind _destination (Variables|Default|GetDestination))
  (bind _returnvalue (Transformation|GetActorLocation _destination))
  (Utilities|FlowControl|DoOnce false) ; enters at Reset
)

(event EventBeginPlay)

(event Collision|EventActorBeginOverlap
  (params (OtherActor :type Actor%20Object%20Reference)))

(event EventTick
  (params (DeltaSeconds :type Float%20%28single-precision%29)))

(fn ConstructionScript)