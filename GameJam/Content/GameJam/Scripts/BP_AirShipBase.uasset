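; Base airship actor with a physics-simulated body, a draining fuel supply and its own destruction sequence.
; BeginPlay loads mass, damping, size and fuel stats from a data table and creates a dynamic material for the fuel gauge.
; Update functions, not called here, toggle physics and flight FX, align rotation to velocity, and drain fuel, refilling it while stopped on a planet.
; DestoryShip runs once, playing an explosion or quick fade; empty fuel triggers the fade and increments the destroyed-ship count.
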(event Custom|DestoryShip
  (params (Bloom :type Boolean))
  (bind _geo1 (Variables|Default|GetGeo1))
  (Utilities|FlowControl|DoOnce false
    (:Completed
      (Variables|Default|SetIsStopPlanet true)
      (Physics|SetSimulatePhysics (Variables|Default|GetPhysicalMesh) false)
      (Rendering|SetVisibility (Variables|Default|GetGeoFule) false false)
      (if Bloom
        (Default|PlayAnim (Variables|Default|GetBPC_MaterialSystem) 1.5 1 10 0 "/Game/GameJam/Texture/T_ShipExplode.T_ShipExplode" _geo1)
        (Audio|PlaySound2D "/Game/GameJam/Sounds/FX/boom.boom" 1.0 1.0 0.0 0 0)
        (Utilities|FlowControl|Delay 1.5)
        (Actor|DestroyActor)
        (else
          (Default|PlayAnimFade (Variables|Default|GetBPC_MaterialSystem) 0.15 _geo1 (Variables|Default|GetShipTexture))
          (Utilities|FlowControl|Delay 0.15)
          (Actor|DestroyActor))))))

(event EventBeginPlay
  (CallFunction|ReadData)
  (Variables|Default|SetFule (Variables|Default|GetMaxFule))
  (bind _returnvalue (Rendering|Material|CreateDynamicMaterialInstance (Variables|Default|GetFuleMaterial) "None" "None" :!class /Script/Engine.KismetMaterialLibrary))
  (Rendering|Material|SetMaterial (Variables|Default|GetGeoFule) 0 _returnvalue))

(event Collision|EventActorBeginOverlap
  (params (OtherActor :type Actor%20Object%20Reference)))

(event EventTick
  (params (DeltaSeconds :type Float%20%28single-precision%29)))

(fn ConstructionScript)

(fn UpdateFule
  (params (Delta :type Float%20%28double-precision%29))
  (if (Variables|Default|GetIsStopPlanet)
    (Variables|Default|SetFule (Variables|Default|GetMaxFule))
    (else
      (Variables|Default|SetFule (Math|Float|Clamp(Float) (- (Variables|Default|GetFule) (* Delta (Variables|Default|GetFuleCostSpeed))) 0.0 (Variables|Default|GetMaxFule)))))
  (bind _as材质动态实例 (Utilities|Casting|CastToMaterialInstanceDynamic (Rendering|Material|GetMaterial (Variables|Default|GetGeoFule) 0))
    (:then
      (Rendering|Material|SetScalarParameterValue _as材质动态实例 "FuleRate" (/ (Variables|Default|GetFule) (Variables|Default|GetMaxFule)) :!class /Script/Engine.MaterialInstanceDynamic))
    (:CastFailed
      _))
  (if (== (Variables|Default|GetFule) 0.0)
    (CallFunction|DestoryShip false)
    (CallFunction|AddAirShipDestroyCount 1)))

(fn UpdateState
  (Physics|SetSimulatePhysics (Variables|Default|GetPhysicalMesh) (not (Variables|Default|GetIsStopPlanet)))
  (Components|Activation|SetActive (Variables|Default|GetFlyFX) (not (Variables|Default|GetIsStopPlanet)) false))

(fn ReadData
  (bind _physicalmesh (Variables|Default|GetPhysicalMesh))
  (bind _returnvalue (Utilities|GetDataTableRow (Variables|Default|GetShipData) "0")
    (:then
      (Variables|Default|SetFuleCostSpeed (.FuleCostPerSecond (Utilities|Struct|BreakST_Ship _returnvalue)))
      (Class|PrimitiveComponent|SetLinearDamping _physicalmesh (.LinearDamping (Utilities|Struct|BreakST_Ship _returnvalue)))
      (Class|PrimitiveComponent|SetAngularDamping _physicalmesh (.AngularDamping (Utilities|Struct|BreakST_Ship _returnvalue)))
      (Class|PrimitiveComponent|SetMassScale _physicalmesh "None" (.Mass (Utilities|Struct|BreakST_Ship _returnvalue)))
      (Transformation|SetRelativeScale3D (Variables|Default|GetPhysicalMesh) (Math|Conversions|ToVector(Float) (.Size (Utilities|Struct|BreakST_Ship _returnvalue))))
      (Variables|Default|SetMaxFule (.FuleMax (Utilities|Struct|BreakST_Ship _returnvalue)))
      (return _returnvalue))))

(fn UpdateRotation
  (if (not (Variables|Default|GetIsStopPlanet))
    (bind _returnvalue (Physics|GetPhysicsLinearVelocity (Variables|Default|GetPhysicalMesh) "None"))
    (Transformation|SetActorRotation (Math|Rotator|Lerp(Rotator) (Math|Rotator|MakeRotfromZ _returnvalue) (Math|Rotator|MakeRotator (.Roll (Math|Rotator|BreakRotator (Math|Rotator|MakeRotfromZ _returnvalue))) (.Pitch (Math|Rotator|BreakRotator (Math|Rotator|MakeRotfromZ _returnvalue))) (+ (.Yaw (Math|Rotator|BreakRotator (Math|Rotator|MakeRotfromZ _returnvalue))) -9e+01)) 1.0))))