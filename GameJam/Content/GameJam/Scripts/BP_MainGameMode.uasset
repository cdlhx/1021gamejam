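; Main game mode that handles level save data, star rating, and victory or defeat for a planet-and-airship game.
; BeginPlay copies saved levels into BP_ChooseGameState, or creates CurrentSaveGame if none exists.
; WriteSaveGame keeps each level's fewest airship losses and best stars, in memory only, without a slot write.
; Airship losses lower stars until defeat below zero; enough upgraded planets mean victory; both endings pause and show a widget.
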(event EventBeginPlay
  (CallFunction|LoadSaveGame))

(fn ConstructionScript)

(fn WriteSaveGame
  (bind _currentsavegame (Variables|Default|GetCurrentSaveGame))
  ;[1 1 1] 保存游戏。在结束某一关卡时调用。
  (bind _asbp_main_game_state (Utilities|Casting|CastToBP_MainGameState (Game|GetGameState)))
  (Utilities|IsValid _currentsavegame
    (:Is%20Valid
      (bind _array_element (Utilities|Array|ForEachLoopwithBreak (Variables|/Game/GameJam/Scripts/LevelLogic/BP_SaveGame.BP_SaveGame_C|GetSavedLevels _currentsavegame) :!label _label)
        (:LoopBody
          ;;[1 1 1] 找到关卡存档，存取分数
          (if (Utilities|Enum|Equal(Enum) (.LevelName (Utilities|Struct|BreakST_LevelData _array_element)) (Utilities|GetObjectName (Class|Actor|GetLevel _asbp_main_game_state)))
            (Utilities|Struct|SetmembersinST_LevelData _array_element (Math|Integer|Min(Integer) (.Score (Utilities|Struct|BreakST_LevelData _array_element)) (Default|GetAirShipDestroyCount _asbp_main_game_state)) (Math|Integer|Max(Integer) (.Star (Utilities|Struct|BreakST_LevelData _array_element)) (Default|GetStar _asbp_main_game_state)))
            (LocalVariables|SetbFindLevel true)
            (goto _label Break)))
        (:Completed
          ;;[1 1 1] 没找到关卡存档，新增一个
          (if (not (LocalVariables|GetbFindLevel))
            (Utilities|Array|Add (Variables|/Game/GameJam/Scripts/LevelLogic/BP_SaveGame.BP_SaveGame_C|GetSavedLevels (Variables|Default|GetCurrentSaveGame)) (Utilities|Struct|MakeST_LevelData (Utilities|GetObjectName (Class|Actor|GetLevel _asbp_main_game_state)) (Default|GetAirShipDestroyCount _asbp_main_game_state) (Default|GetStar _asbp_main_game_state)))))))))

(fn LoadSaveGame
  (bind _returnvalue (SaveGame|DoesSaveGameExist (Variables|Default|GetSaveGameSlot)))
  (if _returnvalue
    (bind _returnvalue_2 (SaveGame|LoadGamefromSlot (Variables|Default|GetSaveGameSlot)))
    ;[1 1 1] 加载所有关卡的分数信息（在选关页面使用，选关页面应使用GameState中的信息）
    (bind _asbp_save_game (Utilities|Casting|CastToBP_SaveGame _returnvalue_2))
    (bind _asbp_choose_game_state (Utilities|Casting|CastToBP_ChooseGameState (Game|GetGameState)))
    (for _array_element (Variables|/Game/GameJam/Scripts/LevelLogic/BP_SaveGame.BP_SaveGame_C|GetSavedLevels _asbp_save_game)
      (Utilities|Array|Add (Variables|/Game/GameJam/Scripts/BP_ChooseGameState.BP_ChooseGameState_C|GetLevelsData _asbp_choose_game_state) _array_element))
    (else
      (bind _returnvalue_3 (SaveGame|CreateSaveGameObject "/Game/GameJam/Scripts/LevelLogic/BP_SaveGame.BP_SaveGame_C"))
      (Variables|Default|SetCurrentSaveGame _returnvalue_3))))

(fn CheckIsVictory
  (bind _outactors (Actor|GetAllActorsOfClass "/Game/GameJam/Scripts/BP_PlanetBase.BP_PlanetBase_C"))
  (for _array_element _outactors
    (if (>= (Variables|/Game/GameJam/Scripts/BP_PlanetBase.BP_PlanetBase_C|GetLevel _array_element) (Variables|Default|GetVictoryStar))
      (Math|Integer|IncrementInt (LocalVariables|GetCount))))
  (return (>= (LocalVariables|GetCount) (Variables|Default|GetVictoryCount))))

(fn CheckIsDefeat
  (return (< (CallFunction|GetStar) 0)))

(fn UpdateStar
  (bind _star (CallFunction|GetStar))
  (if (>= _star 0)
    (if (> (CallFunction|GetAirShipDestroyCount) (Utilities|Array|Get(acopy) (Variables|Default|GetStarDecArray) _star))
      (CallFunction|DecStar)
      (return (CallFunction|GetStar)))))

(fn Victory
  (bind _returnvalue (Game|GetPlayerController 0))
  (Game|SetGamePaused true)
  (Variables|/Script/Engine.PlayerController|SetbShowMouseCursor _returnvalue true)
  (bind _returnvalue_2 (UserInterface|CreateWidget 0 _returnvalue))
  (UserInterface|Viewport|AddtoViewport _returnvalue_2 0))

(fn Defeat
  (bind _returnvalue (Game|GetPlayerController 0))
  (Game|SetGamePaused true)
  (Variables|/Script/Engine.PlayerController|SetbShowMouseCursor _returnvalue true)
  (bind _returnvalue_2 (UserInterface|CreateWidget 0 _returnvalue))
  (UserInterface|Viewport|AddtoViewport _returnvalue_2 0))