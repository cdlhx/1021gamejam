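; Game mode logic that branches on game state to serve both level play and level selection.
; In play, it loads the level's rules from a DataTable and polls each Tick: stars drop as airship losses pass thresholds, enough high-level planets wins, zero stars loses.
; Either result pauses and shows its widget; victory also saves best score and stars if a save object is valid.
; In selection, it loads saved level data into the game state.
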(event EventBeginPlay
  (bind _returnvalue (Game|GetGameState))
  (Utilities|Casting|CastToBP_MainGameState _returnvalue
    (:then
      ;[1 1 1] 加载关卡名对应的信息
      (bind _returnvalue_2 (Game|GetCurrentLevelName true))
      (bind _returnvalue_3 (Utilities|GetDataTableRow (Variables|Default|GetDataTable) (Utilities|String|StringToName _returnvalue_2))
        (:then
          (Variables|Default|SetVictoryCount (.VictoryCount (Utilities|Struct|BreakST_LevelVictotyInfo _returnvalue_3)))
          (Variables|Default|SetVictoryStar (.VictoryStar (Utilities|Struct|BreakST_LevelVictotyInfo _returnvalue_3)))
          (Variables|Default|SetStarDecArray (.StarDecArray (Utilities|Struct|BreakST_LevelVictotyInfo _returnvalue_3))))))
    (:CastFailed
      (Utilities|Casting|CastToBP_ChooseGameState _returnvalue)
      (CallFunction|LoadSaveGame))))

(event EventTick
  (params (DeltaSeconds :type Float%20%28single-precision%29))
  (Utilities|Casting|CastToBP_MainGameState (Game|GetGameState))
  (CallFunction|UpdateStar)
  (bind _isvictory (CallFunction|CheckIsVictory))
  (if _isvictory
    (CallFunction|Victory)
    (else
      (bind _isdefeat (CallFunction|CheckIsDefeat))
      (if _isdefeat
        (CallFunction|Defeat)))))

(fn ConstructionScript)

(fn WriteSaveGame
  (bind _currentsavegame (Variables|Default|GetCurrentSaveGame))
  ;[1 1 1] 保存游戏。在结束某一关卡时调用。
  (bind _asbp_main_game_state (Utilities|Casting|CastToBP_MainGameState (Game|GetGameState)))
  (Utilities|IsValid _currentsavegame
    (:Is%20Valid
      (bind _returnvalue (Game|GetCurrentLevelName true))
      (bind _array_element (Utilities|Array|ForEachLoopwithBreak (Variables|/Game/GameJam/Scripts/LevelLogic/BP_SaveGame.BP_SaveGame_C|GetSavedLevels _currentsavegame) :!label _label)
        (:LoopBody
          ;;[1 1 1] 找到关卡存档，存取分数
          (if (Utilities|Enum|Equal(Enum) (.LevelName (Utilities|Struct|BreakST_LevelData _array_element)) _returnvalue)
            (Utilities|Struct|SetmembersinST_LevelData _array_element (Math|Integer|Min(Integer) (.Score (Utilities|Struct|BreakST_LevelData _array_element)) (Default|GetAirShipDestroyCount _asbp_main_game_state)) (Math|Integer|Max(Integer) (.Star (Utilities|Struct|BreakST_LevelData _array_element)) (Default|GetStar _asbp_main_game_state)))
            (LocalVariables|SetbFindLevel true)
            (goto _label Break)))
        (:Completed
          ;;[1 1 1] 没找到关卡存档，新增一个
          (if (LocalVariables|GetbFindLevel)
            _
            (else
              (Utilities|Array|Add (Variables|/Game/GameJam/Scripts/LevelLogic/BP_SaveGame.BP_SaveGame_C|GetSavedLevels (Variables|Default|GetCurrentSaveGame)) (Utilities|Struct|MakeST_LevelData _returnvalue (Default|GetAirShipDestroyCount _asbp_main_game_state) (Default|GetStar _asbp_main_game_state)))))
          (SaveGame|SaveGametoSlot (Variables|Default|GetCurrentSaveGame) (Variables|Default|GetSaveGameSlot)))))))

(fn LoadSaveGame
  (bind _returnvalue (SaveGame|DoesSaveGameExist (Variables|Default|GetSaveGameSlot)))
  (if _returnvalue
    (bind _returnvalue_2 (SaveGame|LoadGamefromSlot (Variables|Default|GetSaveGameSlot)))
    ;[1 1 1] 加载所有关卡的分数信息（在选关页面使用，选关页面应使用GameState中的信息）
    (bind _asbp_save_game (Utilities|Casting|CastToBP_SaveGame _returnvalue_2))
    (Variables|Default|SetCurrentSaveGame _asbp_save_game)
    (bind _asbp_choose_game_state (Utilities|Casting|CastToBP_ChooseGameState (Game|GetGameState)))
    (for _array_element (Variables|/Game/GameJam/Scripts/LevelLogic/BP_SaveGame.BP_SaveGame_C|GetSavedLevels _asbp_save_game)
      (Utilities|Array|Add (Variables|/Game/GameJam/Scripts/BP_ChooseGameState.BP_ChooseGameState_C|GetLevelsData _asbp_choose_game_state) _array_element))
    (else
      (bind _returnvalue_3 (SaveGame|CreateSaveGameObject "/Game/GameJam/Scripts/LevelLogic/BP_SaveGame.BP_SaveGame_C"))
      (Variables|Default|SetCurrentSaveGame _returnvalue_3))))

(fn CheckIsVictory
  (bind _outactors (Actor|GetAllActorsOfClass "/Game/GameJam/Scripts/BP_PlanetBase.BP_PlanetBase_C"))
  (for _array_element _outactors
    (if (>= (Variables|/Game/GameJam/Scripts/BP_PlanetBase.BP_PlanetBase_C|GetLevel _array_element) (Variables|Default|GetVictoryStar))
      (Math|Integer|IncrementInt (LocalVariables|GetCount))))
  (return (>= (LocalVariables|GetCount) (Variables|Default|GetVictoryCount))))

(fn CheckIsDefeat
  (return (<= (CallFunction|GetStar) 0)))

(fn UpdateStar
  (bind _star (CallFunction|GetStar))
  (if (>= _star 0)
    (if (> (CallFunction|GetAirShipDestroyCount) (Utilities|Array|Get(acopy) (Variables|Default|GetStarDecArray) _star))
      (CallFunction|DecStar)
      (return (CallFunction|GetStar)))))

(fn Victory
  (bind _returnvalue (Game|GetPlayerController 0))
  (Game|SetGamePaused true)
  (CallFunction|WriteSaveGame)
  (Variables|/Script/Engine.PlayerController|SetbShowMouseCursor _returnvalue true)
  (bind _returnvalue_2 (UserInterface|CreateWidget "/Game/GameJam/UI/UI_Victory.UI_Victory_C" _returnvalue))
  (UserInterface|Viewport|AddtoViewport _returnvalue_2 0))

(fn Defeat
  (bind _returnvalue (Game|GetPlayerController 0))
  (Game|SetGamePaused true)
  (Variables|/Script/Engine.PlayerController|SetbShowMouseCursor _returnvalue true)
  (bind _returnvalue_2 (UserInterface|CreateWidget "/Game/GameJam/UI/UI_Defeat.UI_Defeat_C" _returnvalue))
  (UserInterface|Viewport|AddtoViewport _returnvalue_2 0))