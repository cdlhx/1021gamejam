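; BP_MovableShip is a self-propelled ship variant that sets its own ship texture and inherits from a parent Blueprint.
; Each tick it clears CanFly if IsStopPlanet is set, then, while CanFly holds, pushes PhysicalMesh with an X/Y force of current linear velocity plus FlyStrength, so thrust scales with speed.
; Its ReadData override takes FlyStrength from the MoveableFlyStrength field of the parent's data.
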(event Custom|Fly
  (if (Variables|Default|GetCanFly)
    (bind _returnvalue (Physics|GetPhysicsLinearVelocity (Variables|Default|GetPhysicalMesh) "None"))
    (Physics|AddForce (Variables|Default|GetPhysicalMesh) (Math|Vector|MakeVector (.x (+ _returnvalue (Variables|Default|GetFlyStrength))) (.y (+ _returnvalue (Variables|Default|GetFlyStrength))) 0.0) "None" false)))

(event EventBeginPlay
  (|CallParentFunction)
  (Variables|Default|SetShipTexture "/Game/GameJam/Texture/T_MoveableShip.T_MoveableShip"))

(event Collision|EventActorBeginOverlap
  (params (OtherActor :type Actor%20Object%20Reference))
  (|CallParentFunction OtherActor) ; 此节点被禁用，将不会被调用。\n从引脚连出引线来编译功能。
)

(event EventTick
  (params (DeltaSeconds :type Float%20%28single-precision%29))
  (|CallParentFunction DeltaSeconds)
  (CallFunction|UpdateCanFly)
  (CallFunction|Fly))

(fn ConstructionScript
  (|CallParentFunction))

(fn UpdateCanFly
  (if (Variables|Default|GetIsStopPlanet)
    (Variables|Default|SetCanFly false)))

(fn ReadData
  (bind _data (|CallParentFunction))
  (Variables|Default|SetFlyStrength (.Moveable_FlyStrength (Utilities|Struct|BreakST_Ship _data)))
  (return _data))