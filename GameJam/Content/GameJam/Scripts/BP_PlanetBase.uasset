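; Planet actor that starts barren or colonized by Level, configured from a DataTable in the construction script.
; Colonies use looping timers to spawn orbiting ships, launched movable ships and thrown rubbish, rotating orbiters on Tick.
; Incoming higher-level ships reduce ColonyCount; zero colonizes barren planets and raises Level.
; Rubbish entering the outer sphere restores barren planets' count or calls AddAirShipDestroyCount on colonies, which also destroy pirates.
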(event OnComponentBeginOverlap(OuterCircle)
  (params (OverlappedComponent :type Primitive%20Component%20Object%20Reference) (OtherActor :type Actor%20Object%20Reference) (OtherComp :type Primitive%20Component%20Object%20Reference) (OtherBodyIndex :type Integer) (bFromSweep :type Boolean) (SweepResult :type Hit%20Result%20Structure%20%28by%20ref%29))
  (bind _level (Variables|Level|GetLevel))
  (bind _level_2 (Variables|Level|GetLevel))
  (bind _levelupcost (Variables|Level|GetLevelUpCost))
  (bind _update1 (Variables|Default|GetUpdate1))
  (bind _bpc_materialsystem (Variables|Default|GetBPC_MaterialSystem))
  (bind _output (Utilities|Array|Get(acopy) _levelupcost _level_2))
  ;[1 1 1] 处理进入星球的飞船
  (bind _asbp_normal_ship (Utilities|Casting|CastToBP_NormalShip OtherActor)
    (:then
      (if (not (Variables|/Game/GameJam/Scripts/BP_AirShipBase.BP_AirShipBase_C|GetIsStopPlanet _asbp_normal_ship))
        ;[1 1 1] 殖民度减{飞船等级}
        (if (> (Default|GetShipLevel _asbp_normal_ship) (Variables|Level|GetLevel))
          (bind _output_get (Variables|Colony|SetColonyCount (Math|Integer|Clamp(Integer) (- (Variables|Colony|GetColonyCount) (Default|GetShipLevel _asbp_normal_ship)) 0 2147483647)))
          (Default|DestoryShip _asbp_normal_ship true)
          (if (== _output_get 0)
            (if (== (Variables|Level|GetLevel) 0)
              (CallFunction|CasttoColonyPlanet false)
              (Variables|Bool|SetIsColonyPlanet (Variables|Bool|GetIsColonyPlanet)))
            (if (< (Variables|Level|GetLevel) (Utilities|Array|Length _levelupcost))
              (Math|Integer|IncrementInt _level
                (:%20%20
                  (Development|PrintText (Utilities|Text|ToText(Integer) _level))
                  (if (< (Variables|Level|GetLevel) (Utilities|Array|Length (Variables|Level|GetLevelUpCost)))
                    (Variables|Colony|SetMaxColonyCount _output)
                    (Variables|Colony|SetColonyCount _output)
                    (switch int (Variables|Level|GetLevel)
                      (:0
                        (Rendering|SetVisibility _update1 false false :!label _label))
                      (:1
                        (goto _label))
                      (:2
                        (Default|SetMaterial _bpc_materialsystem 2 _update1)
                        (Rendering|SetVisibility _update1 true false :!label _label_2))
                      (:3
                        (Default|SetMaterial _bpc_materialsystem 3 _update1)
                        (goto _label_2)))))))))))
    (:CastFailed
      ;[1 1 1] 处理进入星球的垃圾
      (bind _asbp_rabbish (Utilities|Casting|CastToBP_Rabbish OtherActor)
        (:then
          (Actor|DestroyActor _asbp_rabbish)
          (CallFunction|CollectRabbish))
        (:CastFailed
          ;[1 1 1] 处理进入星球的海盗（缴械）
          (bind _asbp_pirate (Utilities|Casting|CastToBP_Pirate OtherActor))
          (if (Variables|Bool|GetIsColonyPlanet)
            (Actor|DestroyActor _asbp_pirate)))))))

(event Custom|CastToNothingPlanet
  ;[1 1 1] 转换成荒芜星球
  (Variables|Bool|SetIsColonyPlanet false)
  (CallFunction|SpawnShipsAround false)
  (CallFunction|BeginSpawnRabbish false)
  (CallFunction|BeginShipsLeave false)
  (Default|SetMaterial (Variables|Default|GetBPC_MaterialSystem) 1 (Variables|Default|GetGeo)))

(event Custom|CastToColonyPlanet
  (params (First :type Boolean))
  (bind _geo (Variables|Default|GetGeo))
  (bind _bpc_materialsystem (Variables|Default|GetBPC_MaterialSystem))
  ;[1 1 1] 转换成殖民星球
  (Variables|Bool|SetIsColonyPlanet true)
  (CallFunction|SpawnShipsAround true)
  (CallFunction|BeginSpawnRabbish (Variables|Bool|GetIsSpawnRabbish))
  (CallFunction|BeginShipsLeave (Variables|Bool|GetIsSpawnMoveableShip))
  (if First
    (Default|SetMaterial _bpc_materialsystem 0 _geo)
    (else
      (Default|PlayAnim _bpc_materialsystem 3.0 3 10 "/Game/GameJam/Material/MI_ColonyPlanetPlanet.MI_ColonyPlanetPlanet" "/Game/GameJam/Texture/T_Planet_Colonizing.T_Planet_Colonizing" _geo))))

(event Custom|BeginShipsLeave
  (params (Active :type Boolean))
  ;[1 1 1] 动力飞船开始离开
  (if Active
    (bind _returnvalue (Utilities|Time|SetTimerbyEvent (delegate Custom|LeaveOneShip) (Variables|SpawnMovableShips|GetMoveableShipSpawnTime) true))
    (Rendering|SetVisibility (Variables|Default|GetUpdate3) true false)
    (else
      (Utilities|Time|ClearandInvalidateTimerbyHandle _returnvalue))))

(event Custom|SpawnShipsAround
  (params (Active :type Boolean))
  ;[1 1 1] 开始或暂停生成飞船
  (if Active
    (bind _returnvalue (Utilities|Time|SetTimerbyEvent (delegate Custom|SpawnOneShip) (Variables|SpawnShips|GetShipSpawnTime) true))
    (Variables|SpawnShips|SetSpawnShipTimer _returnvalue)
    (else
      (Utilities|Time|ClearandInvalidateTimerbyHandle (Variables|SpawnShips|GetSpawnShipTimer)))))

(event Custom|SpawnOneShip
  ;[1 1 1] 生成一个飞船
  (if (<= (Utilities|Set|Length (Variables|SpawnShips|GetStayAirShips)) (Variables|SpawnShips|GetMaxShipCount))
    (bind _returnvalue (Game|SpawnActorfromClass "/Game/GameJam/Scripts/BP_NormalShip.BP_NormalShip_C" (Math|Transform|MakeTransform (+ (Transformation|GetWorldLocation (Variables|Transformation|GetRootComponent)) (Math|Vector|RotateVector (Math|Vector|MakeVector (Variables|SpawnShips|GetShipsSpawnRadius) 0.0 0.0) (Math|Rotator|MakeRotator 0.0 0.0 (Math|Conversions|ToFloat(Integer) (Math|Random|RandomIntegerinRange 0 360)))))) "Undefined" "MultiplyWithRoot" 0 0))
    (Default|SetShipLevel _returnvalue (Variables|Level|GetLevel))
    (Utilities|Set|Add (Variables|SpawnShips|GetStayAirShips) _returnvalue)
    (Variables|/Game/GameJam/Scripts/BP_AirShipBase.BP_AirShipBase_C|SetIsStopPlanet _returnvalue true)))

(event Custom|LeaveOneShip
  (bind _returnvalue (Math|Random|RandomIntegerinRange 0 360))
  (bind _movableshipsspawnradius (Variables|SpawnMovableShips|GetMovableShipsSpawnRadius))
  (bind _returnvalue_2 (Math|Conversions|ToFloat(Integer) _returnvalue))
  (bind _returnvalue_3 (Math|Vector|MakeVector _movableshipsspawnradius 0.0 0.0))
  (bind _returnvalue_4 (Math|Rotator|MakeRotator 0.0 0.0 _returnvalue_2))
  (bind _returnvalue_5 (Math|Vector|RotateVector _returnvalue_3 _returnvalue_4))
  ;[1 1 1] 一个动力飞船离开
  (bind _returnvalue_6 (Game|SpawnActorfromClass "/Game/GameJam/Scripts/BP_MovableShip.BP_MovableShip_C" (Math|Transform|MakeTransform (+ (Transformation|GetWorldLocation (Variables|Transformation|GetRootComponent)) _returnvalue_5)) "Undefined" "MultiplyWithRoot" 0 0))
  (Utilities|IsValid _returnvalue_6
    (:Is%20Valid
      (Physics|AddForce (Variables|/Game/GameJam/Scripts/BP_AirShipBase.BP_AirShipBase_C|GetPhysicalMesh _returnvalue_6) (* (Class|KismetMathLibrary|VectorNormal2D _returnvalue_5 0.0001) (Variables|SpawnMovableShips|GetMovableShipSpawnForce)) "None" false))))

(event Custom|ShipsMoveAround
  (bind _returnvalue (Transformation|GetActorLocation))
  (bind _removeairships (Variables|Default|GetRemoveAirShips))
  ;[1 1 1] 飞船绕着星球转
  (bind _result (Utilities|Set|ToArray (Variables|SpawnShips|GetStayAirShips)))
  (for _array_element _result
    (Utilities|IsValid _array_element
      (:Is%20Valid
        ;;[1 1 1] 给要移除的飞船放入待移除数组
        (if (Variables|/Game/GameJam/Scripts/BP_AirShipBase.BP_AirShipBase_C|GetIsStopPlanet _array_element)
          (Transformation|SetActorLocation _array_element (+ (Math|Vector|RotateVector (* (Math|Vector|Normalize (- (Transformation|GetActorLocation _array_element) _returnvalue)) (Variables|SpawnShips|GetShipsSpawnRadius)) (Math|Rotator|MakeRotator 0.0 0.0 (Variables|SpawnShips|GetShipsMoveSpeed))) _returnvalue) false false)
          (Transformation|SetActorRotation _array_element (Math|Rotator|FindLookatRotation (* (Math|Vector|Normalize (- (Transformation|GetActorLocation _array_element) _returnvalue)) (Variables|SpawnShips|GetShipsSpawnRadius)) (Math|Vector|RotateVector (* (Math|Vector|Normalize (- (Transformation|GetActorLocation _array_element) _returnvalue)) (Variables|SpawnShips|GetShipsSpawnRadius)) (Math|Rotator|MakeRotator 0.0 0.0 (Variables|SpawnShips|GetShipsMoveSpeed)))))
          (else
            (Utilities|Array|Add (Variables|Default|GetRemoveAirShips) _array_element))))))
  ;;[1 1 1] 移除出轨道的飞船
  (for _array_element_2 _removeairships
    (Utilities|Set|Remove (Variables|SpawnShips|GetStayAirShips) _array_element_2))
  (Utilities|Array|Clear _removeairships))

(event Custom|CollectRabbish
  ;[1 1 1] 收集垃圾
  (if (Variables|Bool|GetIsColonyPlanet)
    (CallFunction|AddAirShipDestroyCount 1)
    (else
      (Variables|Colony|SetColonyCount (Math|Integer|Clamp(Integer) (+ (Variables|Colony|GetColonyCount) 1) 0 (Variables|Colony|GetMaxColonyCount))))))

(event Custom|SpawnRabbish
  (bind _returnvalue (Math|Random|RandomIntegerinRange 0 360))
  (bind _rabbishspawnradius (Variables|SpawnRabbish|GetRabbishSpawnRadius))
  (bind _returnvalue_2 (Math|Conversions|ToFloat(Integer) _returnvalue))
  (bind _returnvalue_3 (Math|Vector|MakeVector _rabbishspawnradius 0.0 0.0))
  (bind _returnvalue_4 (Math|Rotator|MakeRotator 0.0 0.0 _returnvalue_2))
  (bind _returnvalue_5 (Math|Vector|RotateVector _returnvalue_3 _returnvalue_4))
  ;[1 1 1] 生成垃圾
  (Variables|SpawnRabbish|SetSpawnTransform (Math|Transform|MakeTransform (+ (Transformation|GetWorldLocation (Variables|Transformation|GetRootComponent)) _returnvalue_5)))
  (for _index (range 1 (Variables|SpawnRabbish|GetRabbishCountPerSpawn))
    (bind _returnvalue_6 (Game|SpawnActorfromClass "/Game/GameJam/Scripts/BP_Rabbish.BP_Rabbish_C" (Variables|SpawnRabbish|GetSpawnTransform) "AdjustIfPossibleButAlwaysSpawn" "MultiplyWithRoot" 0 0))
    (Utilities|IsValid (Variables|/Game/GameJam/Scripts/BP_AirShipBase.BP_AirShipBase_C|GetPhysicalMesh _returnvalue_6)
      (:Is%20Valid
        (Physics|AddForce (Variables|/Game/GameJam/Scripts/BP_AirShipBase.BP_AirShipBase_C|GetPhysicalMesh _returnvalue_6) (* (Class|KismetMathLibrary|VectorNormal2D _returnvalue_5 0.0001) (Variables|SpawnRabbish|GetThorwForce)) "None" false)))))

(event Custom|BeginSpawnRabbish
  (params (Active :type Boolean))
  ;[1 1 1] 开始生成垃圾
  (if Active
    (if (> (Variables|SpawnRabbish|GetRabbishCountPerSpawn) 0)
      (bind _returnvalue (Utilities|Time|SetTimerbyEvent (delegate Custom|SpawnRabbish) (Variables|SpawnRabbish|GetRabbishSpawnTime) true))
      (Rendering|SetVisibility (Variables|Default|GetUpdate2) true false))
    (else
      (Utilities|Time|ClearandInvalidateTimerbyHandle _returnvalue))))

(event EventBeginPlay
  (bind _level (Variables|Level|GetLevel))
  (bind _levelupcost (Variables|Level|GetLevelUpCost))
  (bind _output (Utilities|Array|Get(acopy) _levelupcost _level))
  (if (< _level 3)
    (Variables|Colony|SetColonyCount _output)
    (Variables|Colony|SetMaxColonyCount _output))
  ;[1 1 1] 如果初始等级为0，转换为荒芜星球，否则转换为殖民星球
  (if (== (Variables|Level|GetLevel) 0)
    (CallFunction|CasttoNothingPlanet)
    (else
      (CallFunction|CasttoColonyPlanet true))))

(event Collision|EventActorBeginOverlap
  (params (OtherActor :type Actor%20Object%20Reference)))

(event EventTick
  (params (DeltaSeconds :type Float%20%28single-precision%29))
  (if (Variables|Bool|GetIsColonyPlanet)
    (CallFunction|ShipsMoveAround)))

(fn ConstructionScript
  (CallFunction|ReadData))

(fn UpdateState
  (bind _bpc_materialsystem (Variables|Default|GetBPC_MaterialSystem))
  (bind _geo (Variables|Default|GetGeo))
  (if (Variables|Bool|GetIsColonyPlanet)
    (Default|SetMaterial _bpc_materialsystem 0 _geo)
    (else
      (Default|SetMaterial _bpc_materialsystem 0 _geo))))

(fn ReadData
  (bind _returnvalue (Utilities|GetDataTableRow (Variables|Default|GetDataTable) "0")
    (:then
      (Transformation|SetRelativeScale3D (Variables|Default|GetGeo) (Math|Conversions|ToVector(Float) (.Size (Utilities|Struct|BreakST_PlaneBase _returnvalue))))
      (Components|Sphere|SetSphereRadius (Variables|Default|GetOuterCircle) (.GetInRadius (Utilities|Struct|BreakST_PlaneBase _returnvalue)) true)
      (Variables|SpawnShips|SetShipsSpawnRadius (.TrackRadius (Utilities|Struct|BreakST_PlaneBase _returnvalue)))
      (Variables|SpawnShips|SetMaxShipCount (.MaxShip (Utilities|Struct|BreakST_PlaneBase _returnvalue)))
      (Variables|SpawnShips|SetShipsMoveSpeed (.ShipMoveAroundSpeed (Utilities|Struct|BreakST_PlaneBase _returnvalue)))
      (Variables|SpawnShips|SetShipSpawnTime (.ShipSpawnTime (Utilities|Struct|BreakST_PlaneBase _returnvalue)))
      (Variables|SpawnMovableShips|SetMoveableShipSpawnTime (.WasteSpawnTime (Utilities|Struct|BreakST_PlaneBase _returnvalue))))))

(fn SetStar
  (params (NewStar :type BP%20Star%20Base%20Object%20Reference))
  (Variables|Default|SetSuroundStar NewStar))

(fn GetStar
  (return (Variables|Default|GetSuroundStar)))