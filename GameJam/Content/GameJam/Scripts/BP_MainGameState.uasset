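; BP_MainGameState is the main game state Blueprint, holding an airship destroy count and a star value.
; Functions add a delta to the destroy count, decrement the star value clamped between zero and three, and return either value.
; It has no active event logic, so both values change only when these functions are called.
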(event EventBeginPlay)

(event EventTick
  (params (DeltaSeconds :type Float%20%28single-precision%29)))

(fn ConstructionScript)

(fn AddAirShipDestroyCount
  (params (Delta :type Integer))
  (Variables|Default|SetAirShipDestroyCount (+ (Variables|Default|GetAirShipDestroyCount) Delta)))

(fn GetAirShipDestroyCount
  (return (Variables|Default|GetAirShipDestroyCount)))

(fn DecStar
  (Variables|Default|SetStar (Math|Integer|Clamp(Integer) (- (Variables|Default|GetStar) 1) 0 3)))

(fn GetStar
  (return (Variables|Default|GetStar)))